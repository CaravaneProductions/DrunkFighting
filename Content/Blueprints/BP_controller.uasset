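; BP_controller is a player controller that handles pausing and holds a health function.
; The Pause input toggles IsPaused, and MenuPause swaps between the PauseMenu and a newly created HUD widget, also switching game pause, cursor and input mode.
; GestionVie calls MortPersonnage on BP_gameMode when damage exceeds Vie; otherwise it adds 1 to Vie, clamped to VieMax, rather than subtracting the damage.
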(event Input|ActionEvents|InputActionPause
  (params (Key :type Key%20Structure))
  ;[1 1 1] Gère la pause dans le jeu
  (:Pressed
    (bind _output_get (Variables|Default|SetIs%20Paused (not (Variables|Default|GetIs%20Paused))))
    (CallFunction|MenuPause _output_get)))

(fn ConstructionScript)

(fn GestionVie
  (params (Dégats :type Float%20%28single-precision%29))
  ;[1 1 1] Vérifie que vie suffisante pour encaisser dégats
  (if (>= (Variables|Default|GetVie) Dégats)
    ;[1 1 1] Si suffisament de points de vie, update la valeur de la vie
    (Variables|Default|SetVie (Math|Float|Clamp(Float) (+ (Variables|Default|GetVie) 1.0) 0.0 (Variables|Default|GetVie%20Max)))
    (else
      (Variables|Default|SetVie 0.0)
      ;[1 1 1] fait mourir le personnage
      (bind _asbp_game_mode (Utilities|Casting|CastToBP_gameMode (Game|GetGameMode)))
      (Default|MortPersonnage _asbp_game_mode self))))

(fn MenuPause
  (params (Is%20Paused :type Boolean))
  ;[1 1 1] Vérifie que le jeu est en pause
  (if Is%20Paused
    ;[1 1 1] met en pause
    (Game|SetGamePaused true)
    (Viewport|RemoveAllWidgets)
    (bind _returnvalue (UserInterface|CreateWidget "/Game/Menus/PauseMenu.PauseMenu_C" self))
    (Variables|/Game/Menus/PauseMenu.PauseMenu_C|SetPlayerWhoPaused _returnvalue 0)
    (UserInterface|Viewport|AddtoViewport _returnvalue 0)
    (Variables|Default|SetbShowMouseCursor true)
    (Input|SetInputModeUIOnly self (Variables|/Game/Menus/PauseMenu.PauseMenu_C|GetButton_continuer _returnvalue) "DoNotLock")
    (else
      ;[1 1 1] enlève la pause
      (Game|SetGamePaused false)
      (Viewport|RemoveAllWidgets)
      (bind _returnvalue_2 (UserInterface|CreateWidget "/Game/Menus/HUD.HUD_C" self))
      (Default|HUDVisibility _returnvalue_2)
      (UserInterface|Viewport|AddtoViewport _returnvalue_2 0)
      (Variables|Default|SetbShowMouseCursor false)
      (Input|SetInputModeGameOnly self))))