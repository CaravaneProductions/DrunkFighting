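; BP_camera is a shared camera that frames up to four players and becomes every BP_controller's view target.
; After a tiny BeginPlay delay it caches the player references from BP_gameMode.
; A fast looping timer sets the spring arm length to the clamped largest pairwise player distance and moves the actor to the players' average position.
; The VInterpTo receives the target as its current value, so movement is unsmoothed.
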(event EventBeginPlay
  ;[1 1 1] pour éviter les conflits
  (Utilities|FlowControl|Delay 0.001)
  ;[1 1 1] fait en sorte que la caméra devienne la caméra de tout le monde
  (CallFunction|ClassSetUp)
  ;[1 1 1] on rafraichit la position du springarm en fonction des joueurs
  (Utilities|Time|SetTimerbyFunctionName 0 "updateCamera" 0.005 true))

(fn ConstructionScript)

(fn ClassSetUp
  ;[1 1 1] On va chercher le tableau des infos des joueurs dans le gamemode
  (bind _asbp_game_mode (Utilities|Casting|CastToBP_gameMode (Game|GetGameMode)))
  (bind _output_get (Variables|Default|SetGame%20Mode _asbp_game_mode))
  (Variables|Default|SetPlayersReference (Variables|/Game/Blueprints/BP_gameMode.BP_gameMode_C|GetPlayers _output_get))
  ;[1 1 1] créée une vue en fonction de chaque controlleur
  (bind _outactors (Actor|GetAllActorsOfClass "/Game/Blueprints/BP_controller.BP_controller_C"))
  (Game|Player|SetViewTargetwithBlend _outactors self 0.0 "VTBlend_Linear" 0.0 false)
  ;[1 1 1] On créée 1 référence pour chaque personnage
  (for (_array_element _array_index) (Variables|Default|GetPlayersReference)
    (switch int _array_index
      (:0
        (Variables|Default|SetP1 _array_element))
      (:1
        (Variables|Default|SetP2 _array_element))
      (:2
        (Variables|Default|SetP3 _array_element))
      (:3
        (Variables|Default|SetP4 _array_element)))))

(fn SetArmLength
  (bind _p1 (Variables|Default|GetP1))
  (bind _p2 (Variables|Default|GetP2))
  (bind _p3 (Variables|Default|GetP3))
  (bind _p4 (Variables|Default|GetP4))
  ;[1 1 1] Va prendre la valeur max de la distance entre les joueurs pour régler la taille du spring arm
  (Variables|/Script/Engine.SpringArmComponent|SetTargetArmLength (Variables|Default|GetSpringArm) (Math|Float|Clamp(Float) (.MaxValue (Math|Float|MaxOfFloatArray (Utilities|Array|MakeArray (CallFunction|CalculateDistance _p1 _p2) (CallFunction|CalculateDistance _p1 _p3) (CallFunction|CalculateDistance _p1 _p4) (CallFunction|CalculateDistance _p2 _p3) (CallFunction|CalculateDistance _p2 _p4) (CallFunction|CalculateDistance _p3 _p4)))) (Variables|armLength|GetminimumArmLength) (Variables|ArmLength|GetmaximumArmLength))))

(fn UpdateCamera
  ;[1 1 1] Adapte le spring arm et la position de la camera
  (CallFunction|SetArmLength)
  (CallFunction|UpdatePosition))

(fn UpdatePosition
  ;[1 1 1] obtient une position moyenne des joueurs et la met dans targetPos
  (Variables|Default|SetTargetPos (/ (+ (CallFunction|GetLocation (Variables|Default|GetP1)) (CallFunction|GetLocation (Variables|Default|GetP2)) (CallFunction|GetLocation (Variables|Default|GetP3)) (CallFunction|GetLocation (Variables|Default|GetP4))) (Utilities|Array|Length (Variables|Default|GetPlayersReference))))
  ;[1 1 1] update la position
  (Transformation|SetActorLocation (Math|Interpolation|VInterpTo (Variables|Default|GetTargetPos) (Variables|Default|GetTargetPos) (Utilities|Time|GetWorldDeltaSeconds) (Variables|Default|GetInterpSpeed)) false false)
  ;[1 1 1] rafraichit la previousPos
  (Variables|Default|SetpreviousPos (Transformation|GetActorLocation)))

(fn GetLocation
  (params (Player :type Actor%20Object%20Reference))
  (Utilities|IsValid Player
    (:Is%20Valid
      (LocalVariables|SetLocation (Transformation|GetActorLocation Player)))
    (:Is%20Not%20Valid
      (LocalVariables|SetLocation "0, 0, 0")))
  (return (LocalVariables|GetLocation)))

(fn CalculateDistance
  (params (player%20Ref%201 :type Actor%20Object%20Reference) (Player%20Ref%202 :type Actor%20Object%20Reference))
  (if (and (Utilities|IsValid player%20Ref%201) (Utilities|IsValid Player%20Ref%202))
    (LocalVariables|SetDistance (Transformation|GetDistanceTo player%20Ref%201 Player%20Ref%202))
    (else
      (LocalVariables|SetDistance 0.0)))
  (return (LocalVariables|GetDistance)))