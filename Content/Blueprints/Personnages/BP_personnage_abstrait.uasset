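; Abstract character Blueprint that sets up health and walk speed at construction, moves along world X from an input axis and destroys itself on lethal damage.
; A box overlap passes abstract item actors to a pickup function, which reads their item structure but is unfinished: the inventory add and item destruction are unconnected.
; The use-item input reads the held item's structure, then clears the reference.
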(event OnComponentBeginOverlap(boiteRecupObjets)
  (params (OverlappedComponent :type Primitive%20Component%20Object%20Reference) (OtherActor :type Actor%20Object%20Reference) (OtherComp :type Primitive%20Component%20Object%20Reference) (OtherBodyIndex :type Integer) (bFromSweep :type Boolean) (SweepResult :type Hit%20Result%20Structure%20%28by%20ref%29))
  (bind _asbp_objets_abstrait (Utilities|Casting|CastToBP_objets_Abstrait OtherActor))
  (CallFunction|RecupObjet _asbp_objets_abstrait))

(event Input|ActionEvents|InputActionUtiliseObjet
  (params (Key :type Key%20Structure))
  ;[1 1 1] Utilisation d'un objet
  (:Pressed
    (Default|GetStructureObjet (Variables|Default|GetobjetRecupere))
    (Variables|Default|SetobjetRecupere 0)))

(event Input|AxisEvents|InputAxisAvancer
  (params (AxisValue :type Float%20%28single-precision%29))
  ;[1 1 1] Mouvement du personnage
  (Pawn|Input|AddMovementInput "1.000000, 0, 0" AxisValue false))

(fn ConstructionScript
  (Variables|Default|Setvie (Variables|Default|GetvieMax))
  (Variables|/Script/Engine.CharacterMovementComponent|SetMaxWalkSpeed (Variables|Character|GetCharacterMovement) (Variables|Default|Getvitesse))
  (Variables|Default|SetpillavePoints 0.0)
  (Variables|Default|SetobjetRecupere 0))

(fn GestionDegats
  (params (degatsRecus :type Float%20%28single-precision%29))
  (if (< degatsRecus (Variables|Default|Getvie))
    (Variables|Default|Setvie (Math|Float|Clamp(Float) (- (Variables|Default|Getvie) degatsRecus) 0.0 (Variables|Default|GetvieMax)))
    (else
      (CallFunction|GestionMort))))

(fn GestionMort
  (Actor|DestroyActor))

(fn RecupObjet
  (params (Objets%20recupere :type BP%20Objets%20Abstrait%20Object%20Reference))
  (Default|GetStructureObjet Objets%20recupere)
  (switch Utilities|FlowControl|Switch|SwitchonE_typeObjets "NewEnumerator0"))