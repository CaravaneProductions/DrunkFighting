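; Game mode for a local multiplayer game that handles player spawning, deaths and random object drops.
; MakeSpawn creates local players, possesses a BP_personnage at each PlayerStart tagged with the player index, and caches all TargetPoints.
; MortPersonnage destroys the dead pawn and awards PillavePoints to its controller, only while NombreMorts is zero.
; Tick uses a Delay and random roll against ChancesSpawnObjet to spawn ObjetChoisi at a random TargetPoint.
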(event Custom|Make%20Spawn
  ;[1 1 1] récupère tous les start points et les met dans un tableau
  (CallFunction|GetPlayerStartPoint)
  ;[1 1 1] fait spawn les joueurs
  (CallFunction|SpawnPlayers)
  (bind _outactors (Actor|GetAllActorsOfClass "/Script/Engine.TargetPoint"))
  (Variables|Default|SetTargetPoint%20list _outactors))

(event Custom|Mort%20Personnage
  (params (player%20controller :type Player%20Controller%20Object%20Reference))
  ;[1 1 1] attribue les pillave points quand le personnage meurt
  (Actor|DestroyActor (Pawn|GetControlledPawn player%20controller))
  (bind _asbp_controller (Utilities|Casting|CastToBP_controller player%20controller))
  (switch int (Variables|Default|GetNombre_morts)
    (:0
      (Variables|/Game/Blueprints/BP_controller.BP_controller_C|SetPillavePoints _asbp_controller (+ (Variables|/Game/Blueprints/BP_controller.BP_controller_C|GetPillavePoints _asbp_controller) 6)))))

(event EventTick
  (params (DeltaSeconds :type Float%20%28single-precision%29))
  (bind _targetpoint_list (Variables|Default|GetTargetPoint%20list))
  ;[1 1 1] Fonction de spawn d'objets
  ;;[1 0.0625 0.0625] Regarde si le tableau existe
  (if (Utilities|Array|IsValidIndex (Variables|Default|GetTargetPoint%20list))
    ;;[1 0.0625 0.0625] ajoute un délai entre deux spawn d'objets
    (Utilities|FlowControl|Delay (Variables|Default|GetTemps%20spawn%20objets))
    ;;[1 0.0625 0.0625] Décide si l'objet spawn
    (if (> (Math|Random|RandomInteger 100) (Variables|Default|GetChances%20spawn%20objet))
      ;;[1 0.0625 0.0625] fait spawn l'objet
      (Game|SpawnActorfromClass (Variables|Default|GetObjet%20choisi) (Transformation|GetActorTransform (Utilities|Array|Get(acopy) _targetpoint_list (Math|Random|RandomInteger (Utilities|Array|Length _targetpoint_list)))) "Undefined" 0 0))))

(fn ConstructionScript)

(fn GetPlayerStartPoint
  ;[1 1 1] récupère tout les player start de la map et les stocke dans un tableau
  (bind _outactors (Actor|GetAllActorsOfClass "/Script/Engine.PlayerStart"))
  (Variables|PlayerAttributes|SetplayerStartArray _outactors))

(fn SpawnPlayers
  ;[1 1 1] Boucle pour le nombre de joueurs
  (for _index (range 0 (- (Variables|PlayerAttributes|GetmaxPlayerCount) 1))
    (Variables|PlayerAttributes|SetIndex _index)
    ;[1 1 1] Pour chaque élément du tableau on regarde s'il est égal à l'index
    (for _array_element (Variables|PlayerAttributes|GetplayerStartArray)
      (if (Utilities|Name|Equal(Name) (Variables|/Script/Engine.PlayerStart|GetPlayerStartTag _array_element) (Utilities|String|StringToName (Utilities|String|ToString(Integer) (Variables|PlayerAttributes|GetIndex))))
        ;[1 1 1] Si tel est le cas, on lui attribue un joueur, un blueprint et un controller
        (Class|GameplayStatics|CreatePlayer (Variables|PlayerAttributes|GetIndex))
        (bind _returnvalue (Game|SpawnActorfromClass "/Game/Blueprints/Perso_no1/BP_personnage.BP_personnage_C" (Transformation|GetActorTransform _array_element) "Undefined" 0 0))
        (Pawn|Possess (Game|GetPlayerController (Variables|PlayerAttributes|GetIndex)) _returnvalue)
        ;[1 1 1] Créée un tableau contenant les informations sur les joueurs
        (Utilities|Array|AddUnique (Variables|PlayerAttributes|GetPlayers) _returnvalue)))))