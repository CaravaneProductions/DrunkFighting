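; Shared camera for two to four players, set as the view target of the player controllers to frame everyone on one screen.
; After BeginPlay, it caches players from BP_gameMode and starts a looping 1 ms timer calling UpdateCamera.
; Each update moves it to the players' average position and sets spring arm length to their largest pairwise distance, clamped.
; VInterpTo receives TargetPos as both current and target, so movement is unsmoothed.
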(event EventBeginPlay
  ;[1 1 1] pour éviter les conflits
  (Utilities|FlowControl|Delay 0.001)
  ;[1 1 1] fait en sorte que la caméra devienne la caméra de tout le monde
  (CallFunction|ClassSetUp)
  ;[1 1 1] on rafraichit la position du springarm en fonction des joueurs
  (Utilities|Time|SetTimerbyFunctionName 0 "updateCamera" 0.001 true))

(fn ConstructionScript)

(fn ClassSetUp
  ;[1 1 1] On va chercher le tableau des infos des joueurs dans le gamemode
  (bind _asbp_game_mode (Utilities|Casting|CastToBP_gameMode (Game|GetGameMode)))
  (bind _output_get (Variables|Default|SetGame%20Mode _asbp_game_mode))
  (Variables|Default|SetPlayersReference (Variables|/Game/Personnage/BP_gameMode.BP_gameMode_C|GetPlayers _output_get))
  ;[1 1 1] créée une vue en fonction de chaque controlleur
  (bind _outactors (Actor|GetAllActorsOfClass "/Script/Engine.PlayerController"))
  (Game|Player|SetViewTargetwithBlend _outactors self 0.0 "VTBlend_Linear" 0.0 false)
  ;[1 1 1] On créée 1 référence pour chaque personnage
  (for (_array_element _array_index) (Variables|Default|GetPlayersReference)
    (switch int _array_index
      (:0
        (Variables|Default|SetP1 _array_element))
      (:1
        (Variables|Default|SetP2 _array_element))
      (:2
        (Variables|Default|SetP3 _array_element))
      (:3
        (Variables|Default|SetP4 _array_element)))))

(fn SetArmLengthP4
  (bind _p1 (Variables|Default|GetP1))
  (bind _p2 (Variables|Default|GetP2))
  (bind _p3 (Variables|Default|GetP3))
  (bind _p4 (Variables|Default|GetP4))
  ;[1 1 1] Va prendre la valeur max de la distance entre les joueurs pour régler la taille du spring arm
  (Variables|/Script/Engine.SpringArmComponent|SetTargetArmLength (Variables|Default|GetSpringArm) (Math|Float|Clamp(Float) (.MaxValue (Math|Float|MaxOfFloatArray (Utilities|Array|MakeArray (Transformation|GetDistanceTo _p1 _p2) (Transformation|GetDistanceTo _p1 _p3) (Transformation|GetDistanceTo _p1 _p4) (Transformation|GetDistanceTo _p2 _p3) (Transformation|GetDistanceTo _p2 _p4) (Transformation|GetDistanceTo _p3 _p4)))) (Variables|armLength|GetminimumArmLength) (Variables|ArmLength|GetmaximumArmLength))))

(fn SetArmLengthP3
  (bind _p1 (Variables|Default|GetP1))
  (bind _p2 (Variables|Default|GetP2))
  (bind _p3 (Variables|Default|GetP3))
  ;[1 1 1] Va prendre la valeur max de la distance entre les joueurs pour régler la taille du spring arm
  (Variables|/Script/Engine.SpringArmComponent|SetTargetArmLength (Variables|Default|GetSpringArm) (Math|Float|Clamp(Float) (.MaxValue (Math|Float|MaxOfFloatArray (Utilities|Array|MakeArray (Transformation|GetDistanceTo _p1 _p2) (Transformation|GetDistanceTo _p1 _p3) (Transformation|GetDistanceTo _p2 _p3)))) (Variables|armLength|GetminimumArmLength) (Variables|ArmLength|GetmaximumArmLength))))

(fn SetArmLengthP2
  ;[1 1 1] Va prendre la valeur max de la distance entre les joueurs pour régler la taille du spring arm
  (Variables|/Script/Engine.SpringArmComponent|SetTargetArmLength (Variables|Default|GetSpringArm) (Math|Float|Clamp(Float) (Transformation|GetDistanceTo (Variables|Default|GetP1) (Variables|Default|GetP2)) (Variables|armLength|GetminimumArmLength) (Variables|ArmLength|GetmaximumArmLength))))

(fn UpdateCamera
  ;[1 1 1] selon le nombre de joueurs en jeu
  (switch int (Utilities|Array|Length (Variables|Default|GetPlayersReference))
    (:2
      ;[1 1 1] choisit une des facons de jouer sur le spring arm
      (CallFunction|SetArmLengthP2)
      (CallFunction|UpdatePositionP2))
    (:3
      (CallFunction|SetArmLengthP3)
      (CallFunction|UpdatePositionP3))
    (:4
      (CallFunction|SetArmLengthP4)
      (CallFunction|UpdatePositionP4))))

(fn UpdatePositionP4
  ;[1 1 1] obtient une position moyenne des joueurs et la met dans targetPos
  (Variables|Default|SetTargetPos (/ (+ (Transformation|GetActorLocation (Variables|Default|GetP1)) (Transformation|GetActorLocation (Variables|Default|GetP2)) (Transformation|GetActorLocation (Variables|Default|GetP3)) (Transformation|GetActorLocation (Variables|Default|GetP4))) (Utilities|Array|Length (Variables|Default|GetPlayersReference))))
  ;[1 1 1] update la position
  (Transformation|SetActorLocation (Math|Interpolation|VInterpTo (Variables|Default|GetTargetPos) (Variables|Default|GetTargetPos) (Utilities|Time|GetWorldDeltaSeconds) (Variables|Default|GetInterpSpeed)) false false)
  ;[1 1 1] rafraichit la previousPos
  (Variables|Default|SetpreviousPos (Transformation|GetActorLocation)))

(fn UpdatePositionP3
  ;[1 1 1] obtient une position moyenne des joueurs et la met dans targetPos
  (Variables|Default|SetTargetPos (/ (+ (Transformation|GetActorLocation (Variables|Default|GetP1)) (Transformation|GetActorLocation (Variables|Default|GetP2)) (Transformation|GetActorLocation (Variables|Default|GetP3))) (Utilities|Array|Length (Variables|Default|GetPlayersReference))))
  ;[1 1 1] update la position
  (Transformation|SetActorLocation (Math|Interpolation|VInterpTo (Variables|Default|GetTargetPos) (Variables|Default|GetTargetPos) (Utilities|Time|GetWorldDeltaSeconds) (Variables|Default|GetInterpSpeed)) false false)
  ;[1 1 1] rafraichit la previousPos
  (Variables|Default|SetpreviousPos (Transformation|GetActorLocation)))

(fn UpdatePositionP2
  ;[1 1 1] obtient une position moyenne des joueurs et la met dans targetPos
  (Variables|Default|SetTargetPos (/ (+ (Transformation|GetActorLocation (Variables|Default|GetP1)) (Transformation|GetActorLocation (Variables|Default|GetP2))) (Utilities|Array|Length (Variables|Default|GetPlayersReference))))
  ;[1 1 1] update la position
  (Transformation|SetActorLocation (Math|Interpolation|VInterpTo (Variables|Default|GetTargetPos) (Variables|Default|GetTargetPos) (Utilities|Time|GetWorldDeltaSeconds) (Variables|Default|GetInterpSpeed)) false false)
  ;[1 1 1] rafraichit la previousPos
  (Variables|Default|SetpreviousPos (Transformation|GetActorLocation)))