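; BP_gameMode is a game mode that spawns the local players when play begins.
; It gathers every PlayerStart in the map, then for each index up to MaxPlayerCount finds the starts whose PlayerStartTag matches that index.
; At a matching start it creates the local player, spawns a BP_PersonnageTest, possesses it with that player's controller and adds the pawn to the Players array.
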(event EventBeginPlay
  ;[1 1 1] récupère tous les start points et les met dans un tableau
  (CallFunction|GetPlayerStartPoint)
  ;[1 1 1] fait spawn les joueurs
  (CallFunction|SpawnPlayers))

(fn ConstructionScript)

(fn GetPlayerStartPoint
  ;[1 1 1] récupère tout les player start de la map et les stocke dans un tableau
  (bind _outactors (Actor|GetAllActorsOfClass "/Script/Engine.PlayerStart"))
  (Variables|PlayerAttributes|SetplayerStartArray _outactors))

(fn SpawnPlayers
  ;[1 1 1] Boucle pour le nombre de joueurs
  (for _index (range 0 (- (Variables|PlayerAttributes|GetmaxPlayerCount) 1))
    (Variables|PlayerAttributes|SetIndex _index)
    ;[1 1 1] Pour chaque élément du tableau on regarde s'il est égal à l'index
    (for _array_element (Variables|PlayerAttributes|GetplayerStartArray)
      (if (Utilities|Name|Equal(Name) (Variables|/Script/Engine.PlayerStart|GetPlayerStartTag _array_element) (Utilities|String|StringToName (Utilities|String|ToString(Integer) (Variables|PlayerAttributes|GetIndex))))
        ;[1 1 1] Si tel est le cas, on lui attribue un joueur, un blueprint et un controller
        (Class|GameplayStatics|CreatePlayer (Variables|PlayerAttributes|GetIndex))
        (bind _returnvalue (Game|SpawnActorfromClass "/Game/Personnage/BP_PersonnageTest.BP_PersonnageTest_C" (Transformation|GetActorTransform _array_element) "Undefined" 0 0))
        (Pawn|Possess (Game|GetPlayerController (Variables|PlayerAttributes|GetIndex)) _returnvalue)
        ;[1 1 1] Créée un tableau contenant les informations sur les joueurs
        (Utilities|Array|AddUnique (Variables|PlayerAttributes|GetPlayers) _returnvalue)))))